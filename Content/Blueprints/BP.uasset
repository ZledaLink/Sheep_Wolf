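; Blueprint that positions a camera along a spline, apparently as a camera rail.
; Each Tick sets the camera's relative transform from a distance of frame delta times SplineSpeed, which does not accumulate.
; When the camera nears spline point 1, it sets Stopped and halts a Timeline, whose updates place the camera at spline length plus an offset.
; Left key plays the Timeline and clears Stopped after a short delay.
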(event `self.ReceiveTick`
  (params (DeltaSeconds :type "Float (single-precision)"))
  (bind _returnvalue (`SplineComponent.GetTransformAtDistanceAlongSpline` (`self.Spline`) (`self.DistanceAlongSpline`) "Local" false))
  (set `self.DistanceAlongSpline` (+ (* DeltaSeconds (`self.SplineSpeed`)) 0.0))
  (`SceneComponent.K2_SetRelativeTransform` (`self.Camera`) (`KismetMathLibrary.MakeTransform` (.location _returnvalue) (`KismetMathLibrary.MakeRotator` (.roll (.rotation _returnvalue)) (.pitch (.rotation _returnvalue)) (+ (.yaw (.rotation _returnvalue)) 0.0)) (`SceneComponent.RelativeScale3D` (`self.Camera`))) false false)
  (if (`self.Stopped`)
    _
    (elif (`KismetMathLibrary.NearlyEqual_TransformTransform` (`SceneComponent.GetRelativeTransform` (`self.Camera`)) (`SplineComponent.GetTransformAtSplinePoint` (`self.Spline`) 1 "Local" false) 0.0001 10.0 10.0)
      (set `self.Stopped` true)
      (bind (_direction _0_1) (`Timeline|Timeline` :!via `Stop` :!label _label)
        (:`Update`
          (`SceneComponent.K2_SetRelativeTransform` (`self.Camera`) (`SplineComponent.GetTransformAtDistanceAlongSpline` (`self.Spline`) (+ (`SplineComponent.GetSplineLength` (`self.Spline`)) _0_1) "Local" false) false false))))))

(event `ResetStop`
  (`KismetSystemLibrary.Delay` 0.25)
  (set `self.Stopped` false))

(event `Key|Left`
  (params (Key :type "Key Structure"))
  (:`Pressed`
    (`self.ResetStop`)
    (goto _label)))

(fn `UserConstructionScript`)